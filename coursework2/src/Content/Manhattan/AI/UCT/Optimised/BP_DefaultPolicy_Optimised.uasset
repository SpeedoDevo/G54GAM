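; Default rollout policy for the UCT game AI in Manhattan, playing a given game state forward with greedy moves until it ends or hits a depth limit.
; Moves are applied in batches with a zero-length Delay between them, keeping simulations fast without blocking the game.
; The result is reported as a two-player reward vector: a full point to the winner, or half each when the game is unfinished.
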(event `self.OnApply`
  (params (Game :type "/Game/Manhattan/Core/Data/SGameState Structure"))
  (bind _currentstate_phase (break `/Game/Manhattan/Core/Data/SGameState` (`self.CurrentState`)))
  (set `self.CurrentState` Game)
  (set `self.Depth` 0)
  ;[1 1 1] while the state is
  ; non-terminal
  (if (not (`|EnumEquality` "NewEnumerator3" _currentstate_phase)) :!label _label
    ;[1 1 1] apply a random greedy move
    (bind _moves (`/Game/Manhattan/Core/Rules/BPFL_Rules.GetPossibleMoves` (`self.CurrentState`)))
    (bind _move (`/Game/Manhattan/Core/Rules/BPFL_Rules.GreedyMove` _moves (`self.CurrentState`)))
    (bind _newgame (`/Game/Manhattan/Core/Rules/BPFL_Rules.ApplyMove` (`self.CurrentState`) _move))
    (set `self.CurrentState` _newgame)
    ;[1 1 1] if depth limit is reached then terminate, winner is unknown
    (bind _result (`/Engine/EditorBlueprintResources/StandardMacros.IncrementInt` (`self.Depth`))
      (:`  `
        (if (>= _result (`self.MaxDepth`))
          _
          (else
            ;[1 1 1] apply n moves before delaying
            (if (!= (mod (`self.Depth`) (`self.ApplyInOneGoCount`)) 0)
              (goto _label)
              (else
                (`KismetSystemLibrary.Delay` 0.0) ; ensure non-blocking
                (goto _label))))))))
  ;[1 1 1] evaluate winner
  (`self.OnApplyResult` (`self.GetRewardValue` (`self.CurrentState`))))

(fn `GetRewardValue`
  (params (Game :type "/Game/Manhattan/Core/Data/SGameState Structure (by ref)"))
  (returns (Value :type "Vector Structure"))
  (if (`|EnumEquality` Game_Phase_34_EA611F984BA0D790EF2F2DBB9B103858 "NewEnumerator3")
    (if (`|EnumEquality` "NewEnumerator0" Game_WinningPlayer_39_5310132F436322AFA826B69CF7728160)
      (return (1.0 0.0 0.0))
      (else
        (return (0.0 1.0 0.0))))
    (else
      (return (0.5 0.5 0.0)))))

(fn `UserConstructionScript`
  (`parent.UserConstructionScript`))