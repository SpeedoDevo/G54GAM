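; An optimised UCT (Monte Carlo tree search) AI controller that runs simulations to search game states.
; It spawns optimised tree and default policy actors, passing the latter a depth limit and batch size from FrameRateTradeoff.
; The tree persists between turns: selected moves promote the matching child to root, or clear the tree if unexplored.
; Each search runs only enough simulations to lift root visits to TargetConfidence, reporting progress as a fraction.
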(event `self.ReceiveBeginPlay`
  ;[1 1 1] create the policies
  (bind _returnvalue (`|SpawnActorFromClass` "/Game/Manhattan/AI/UCT/Optimised/BP_TreePolicy_Optimised.BP_TreePolicy_Optimised_C" (`KismetMathLibrary.MakeTransform` (0.0 0.0 0.0)) "Undefined" "OverrideRootScale" self null))
  (set `self.TreePolicy` _returnvalue)
  (bind _returnvalue_2 (`|SpawnActorFromClass` "/Game/Manhattan/AI/UCT/Optimised/BP_DefaultPolicy_Optimised.BP_DefaultPolicy_Optimised_C" (`KismetMathLibrary.MakeTransform` (0.0 0.0 0.0)) "Undefined" "OverrideRootScale" self (`self.MaxDepth`) (`self.FrameRateTradeoff`) null))
  (set `self.DefaultPolicy` _returnvalue_2)
  (`parent.ReceiveBeginPlay`))

(event `self.OnSearch`
  (params (Game :type "/Game/Manhattan/Core/Data/SGameState Structure (by ref)"))
  (bind (_node_move _node_state _node_untriedmoves _node_visits) (break `/Game/Manhattan/AI/GameTree/SGameTreeNode` (`/Game/Manhattan/AI/GameTree/BP_GameTree.Node` (`self.Root`))))
  (`self.SetRootIfNeeded` Game) ; only create a new root if an unexplored state is being searched
  (set `self.SimulationCount` 0)
  (set `self.MaxSimulations` (- (`self.TargetConfidence`) _node_visits))
  (`self.OnCheckBudget`))

(event `self.OnCheckBudget`
  (if (< (`self.SimulationCount`) (`self.MaxSimulations`))
    (`self.OnWithinBudget`)
    (else
      (`self.OnOutOfBudget`))))

(event `self.OnSimulationFinished`
  (`/Engine/EditorBlueprintResources/StandardMacros.IncrementInt` (`self.SimulationCount`)))

(event `self.OnMoveSelected`
  (params (Move :type "/Game/Manhattan/Core/Data/SMove Structure"))
  (`self.OnAdvanceTree` Move) ; use opponents move to keep the search tree updated
)

(event `OnAdvanceTree`
  (params (Move :type "/Game/Manhattan/Core/Data/SMove Structure"))
  (bind _root (`self.Root`)
    (:`then`
      (bind (_value _returnvalue) (`BlueprintMapLibrary.Map_Find` (`/Game/Manhattan/AI/GameTree/BP_GameTree.Children` _root) Move))
      (if _returnvalue
        ;[1 1 1] set it as the new root by clearing its parent reference
        (bind _output_get (set `self.Root` _value))
        (set `/Game/Manhattan/AI/GameTree/BP_GameTree.Parent` null _output_get)
        (else
          (set `self.Root` null) ; move unexplored\nclear the game tree\nnew one will be created on next search
        )))
    (:`else`)))

(fn `GetProgress`
  (returns (Progress :type "Float (double-precision)"))
  (return (/ (`KismetMathLibrary.Conv_IntToDouble` (`self.SimulationCount`)) (`KismetMathLibrary.Conv_IntToDouble` (`self.MaxSimulations`)))))

(fn `SetRootIfNeeded`
  (params (Game :type "/Game/Manhattan/Core/Data/SGameState Structure (by ref)"))
  (`self.Root`
    (:`then`
      (return))
    (:`else`
      (bind _root (`self.MakeRoot` Game))
      (set `self.Root` _root)
      (return))))

(fn `UserConstructionScript`
  (`parent.UserConstructionScript`))