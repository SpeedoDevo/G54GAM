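; Tree policy for UCT Monte Carlo tree search in the Manhattan game AI, selecting the node to evaluate next.
; OnApply descends through fully expanded nodes via BestChild, yielding with a zero Delay each level, then returns a terminal node or new expansion through CallOnApplyResult.
; BestChild scores children with a UCB1 math expression using the reward of the parent's current player, breaking ties randomly.
; DebugTree prints node statistics.
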(event EventOnApply
  (params (Tree :type BP%20Game%20Tree%20Object%20Reference) (ExplorationFactor :type Float%20%28single-precision%29))
  (Variables|Default|SetCurrentTree Tree)
  ;[1 1 1] while current tree is non-terminal
  (if (Default|IsTerminal (Variables|Default|GetCurrentTree)) :!label _label
    (Default|CallOnApplyResult (Variables|Default|GetCurrentTree))
    (else
      ;[1 1 1] and not fully expanded
      (if (Default|IsFullyExpanded (Variables|Default|GetCurrentTree))
        ;[1 1 1] not expandable so dig deeper in the tree
        (bind _child (CallFunction|BestChild (Variables|Default|GetCurrentTree) ExplorationFactor))
        (Variables|Default|SetCurrentTree _child)
        (Utilities|FlowControl|Delay 0.0)
        (goto _label)
        (else
          ;[1 1 1] expandable so return an expansion
          (bind _child_2 (Default|Expand (Variables|Default|GetCurrentTree)))
          (Default|CallOnApplyResult _child_2))))))

(fn ConstructionScript
  (|CallParentFunction))

(fn ChildValue
  (params (Child :type BP%20Game%20Tree%20Object%20Reference) (ExplorationFactor :type Float%20%28single-precision%29))
  (bind (_rules _parent _children _node) (Default|Split Child))
  (bind _node_2 (Variables|/Game/Manhattan/AI/GameTree/BP_GameTree.BP_GameTree_C|GetNode _parent))
  (return (|((Reward/Visits)+(ExplorationFactor*(sqrt(((2*(loge(ParentVisits)))/Visits))))) ExplorationFactor (Math|Conversions|ToFloat(Integer) (.visits _node)) (Math|Conversions|ToFloat(Integer) (.visits _node_2)) (Utilities|Select :Index (.currentplayer (.state _node_2)) :NewEnumerator0 (.x (.reward _node)) :NewEnumerator1 (.y (.reward _node))))))

(fn BestChild
  (params (Tree :type BP%20Game%20Tree%20Object%20Reference) (ExplorationFactor :type Float%20%28single-precision%29))
  ;[1 1 1] for each child node
  (bind _values (Utilities|Map|Values (Variables|/Game/Manhattan/AI/GameTree/BP_GameTree.BP_GameTree_C|GetChildren Tree)))
  (for _array_element _values
    (bind _output_get (LocalVariables|SetCurrentChild _array_element))
    (bind _value (CallFunction|ChildValue _output_get ExplorationFactor))
    ;[1 1 1] if value is as good as the best known value then add it to the list
    (if (== _value (LocalVariables|GetBestValue))
      (Utilities|Array|Add (LocalVariables|GetMaxs) (LocalVariables|GetCurrentChild))
      (else
        ;[1 1 1] if value is better than the best known then restart the list
        (if (> _value (LocalVariables|GetBestValue))
          (LocalVariables|SetBestValue _value)
          (LocalVariables|SetMaxs (Utilities|Array|MakeArray (LocalVariables|GetCurrentChild)))))))
  (return (Utilities|Array|Get(acopy) (LocalVariables|GetMaxs) (Math|Random|RandomIntegerinRange 0 (Utilities|Array|LastIndex (LocalVariables|GetMaxs))))))

(fn DebugTree
  (params (Tree :type BP%20Game%20Tree%20Object%20Reference) (TextColor :type Linear%20Color%20Structure) (ExplorationFactor :type Float%20%28single-precision%29))
  (bind (_rules _parent _children _node) (Default|Split Tree))
  (Utilities|IsValid _parent
    (:Is%20Valid
      (bind _value (CallFunction|ChildValue Tree ExplorationFactor)))
    (:Is%20Not%20Valid
      _))
  (Development|PrintString (Utilities|String|Append (Utilities|String|ToString(Integer) (.visits _node)) "      " (Utilities|String|ToString(Vector) (.reward _node)) "      " (Utilities|String|ToString(Float) _value) "      " (CallFunction|MovetoString (.move _node))) true true TextColor 1e+01))