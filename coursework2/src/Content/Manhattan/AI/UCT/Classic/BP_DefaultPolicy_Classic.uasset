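; Default policy for the classic UCT AI in Manhattan, playing a random rollout from a given game state to the terminal phase.
; Each iteration applies a uniformly random possible move, with a zero-length Delay spreading the loop across frames to avoid blocking.
; At the end, GetRewardValue turns the winning player into a win-or-loss reward vector, passed on through CallOnApplyResult.
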(event `self.OnApply`
  (params (Game :type "/Game/Manhattan/Core/Data/SGameState Structure"))
  (bind _currentstate_phase (break `/Game/Manhattan/Core/Data/SGameState` (`self.CurrentState`)))
  (set `self.CurrentState` Game)
  ;[1 1 1] while the state is
  ; non-terminal
  (if (`|EnumEquality` "NewEnumerator3" _currentstate_phase) :!label _label
    ;[1 1 1] evaluate winner
    (`self.OnApplyResult` (`self.GetRewardValue` (`self.CurrentState`)))
    (else
      ;[1 1 1] apply a random move
      (bind _moves (`/Game/Manhattan/Core/Rules/BPFL_Rules.GetPossibleMoves` (`self.CurrentState`)))
      (bind _newgame (`/Game/Manhattan/Core/Rules/BPFL_Rules.ApplyMove` (`self.CurrentState`) (`|GetArrayItem` _moves (`KismetMathLibrary.RandomIntegerInRange` 0 (`KismetArrayLibrary.Array_LastIndex` _moves)))))
      (set `self.CurrentState` _newgame)
      (`KismetSystemLibrary.Delay` 0.0) ; ensure non-blocking
      (goto _label))))

(fn `GetRewardValue`
  (params (Game :type "/Game/Manhattan/Core/Data/SGameState Structure (by ref)"))
  (returns (Value :type "Vector Structure"))
  (if (`|EnumEquality` "NewEnumerator0" Game_WinningPlayer_39_5310132F436322AFA826B69CF7728160)
    (return (1.0 0.0 0.0))
    (else
      (return (0.0 1.0 0.0)))))

(fn `UserConstructionScript`
  (`parent.UserConstructionScript`))