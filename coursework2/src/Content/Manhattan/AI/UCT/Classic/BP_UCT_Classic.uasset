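; BP_UCT_Classic is the classic variant of the UCT search AI in the Manhattan game, extending a parent search Blueprint.
; On BeginPlay it spawns classic tree and default policy actors and assigns them for the search.
; Each search resets a simulation counter, and the budget check reports out of budget once that counter passes a hardcoded limit.
; SetBudget stores a value that this check ignores.
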(event `self.ReceiveBeginPlay`
  ;[1 1 1] create the policies
  (bind _returnvalue (`|SpawnActorFromClass` "/Game/Manhattan/AI/UCT/Classic/BP_TreePolicy_Classic.BP_TreePolicy_Classic_C" (`KismetMathLibrary.MakeTransform` (0.0 0.0 0.0)) "Undefined" "OverrideRootScale" self null))
  (set `self.TreePolicy` _returnvalue)
  (bind _returnvalue_2 (`|SpawnActorFromClass` "/Game/Manhattan/AI/UCT/Classic/BP_DefaultPolicy_Classic.BP_DefaultPolicy_Classic_C" (`KismetMathLibrary.MakeTransform` (0.0 0.0 0.0)) "Undefined" "OverrideRootScale" self null))
  (set `self.DefaultPolicy` _returnvalue_2)
  (`parent.ReceiveBeginPlay`))

(event `self.OnSearch`
  (params (Game :type "/Game/Manhattan/Core/Data/SGameState Structure (by ref)"))
  ;[1 1 1] do 100 simulations every time search is called
  (set `self.SimulationCount` 0)
  (`parent.OnSearch` Game))

(event `self.OnCheckBudget`
  ;[1 1 1] do 100 simulations every time search is called
  (if (<= (`self.SimulationCount`) 100)
    (`self.OnWithinBudget`)
    (else
      (`self.OnOutOfBudget`))))

(event `self.OnSimulationFinished`
  ;[1 1 1] do 100 simulations every time search is called
  (`/Engine/EditorBlueprintResources/StandardMacros.IncrementInt` (`self.SimulationCount`)))

(fn `SetBudget`
  (params (Budget :type Integer))
  (set `self.Budget` Budget)
  (return))

(fn `UserConstructionScript`
  (`parent.UserConstructionScript`))