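; Base Blueprint for a UCT Monte Carlo tree search that selects an AI move from a given game state.
; Each iteration, the tree policy picks a node, the default policy simulates from it, and the reward is backed up.
; A zero Delay between iterations keeps the search non-blocking.
; Empty budget hooks are left for overriding; once out of budget, it reports the best root child with zero exploration.
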(event `self.ReceiveBeginPlay`
  (set `self.RulesDelegate` (`self.MakeRulesDelegate`)) ; all created root nodes should have the same delegate
  (add `/Game/Manhattan/AI/UCT/Base/BP_TreePolicy.OnApplyResult` (`self.TreePolicy`) (delegate `OnTreePolicyResult`))
  (add `/Game/Manhattan/AI/UCT/Base/BP_DefaultPolicy.OnApplyResult` (`self.DefaultPolicy`) (delegate `OnDefaultPolicyResult`)))

(event `OnSearch`
  (params (Game :type "/Game/Manhattan/Core/Data/SGameState Structure (by ref)"))
  ;[1 1 1] create a new root node and start search
  (bind _root (`self.MakeRoot` Game))
  (set `self.Root` _root)
  (`self.OnCheckBudget`))

(event `OnCheckBudget`)

(event `OnWithinBudget`
  (`self.OnSimulate`))

(event `OnSimulate`
  (`/Game/Manhattan/AI/UCT/Base/BP_TreePolicy.OnApply` (`self.TreePolicy`) (`self.Root`) (`self.ExplorationFactor`)))

(event `OnTreePolicyResult`
  (params (Child :type "/Game/Manhattan/AI/GameTree/BP_GameTree Object Reference"))
  (bind _output_get (set `self.CurrentTree` Child))
  (bind (_node_move _node_state) (break `/Game/Manhattan/AI/GameTree/SGameTreeNode` (`/Game/Manhattan/AI/GameTree/BP_GameTree.Node` _output_get)))
  (`/Game/Manhattan/AI/UCT/Base/BP_DefaultPolicy.OnApply` (`self.DefaultPolicy`) _node_state))

(event `OnDefaultPolicyResult`
  (params (Reward :type "Vector Structure"))
  (`/Game/Manhattan/AI/GameTree/BP_GameTree.BackupMonteCarlo` (`self.CurrentTree`) Reward)
  (`self.OnSimulationFinished`)
  (`KismetSystemLibrary.Delay` 0.0) ; ensure that the search is non-blocking
  (`self.OnCheckBudget`) ; check if more searches are needed
)

(event `OnSimulationFinished`)

(event `OnOutOfBudget`
  (bind _child (`/Game/Manhattan/AI/UCT/Base/BP_TreePolicy.BestChild` (`self.TreePolicy`) (`self.Root`) 0.0))
  (bind _node_move (break `/Game/Manhattan/AI/GameTree/SGameTreeNode` (`/Game/Manhattan/AI/GameTree/BP_GameTree.Node` _child)))
  (`self.OnMoveSelected` _node_move)
  (`self.OnSearchComplete` _node_move))

(event `OnMoveSelected`
  (params (Move :type "/Game/Manhattan/Core/Data/SMove Structure")))

(fn `MakeRoot`
  (params (Game :type "/Game/Manhattan/Core/Data/SGameState Structure (by ref)"))
  (returns (Root :type "/Game/Manhattan/AI/GameTree/BP_GameTree Object Reference"))
  (bind _moves (`/Game/Manhattan/Core/Rules/BPFL_Rules.GetPossibleMoves` Game))
  (bind _returnvalue (`|GenericCreateObject` "/Game/Manhattan/AI/GameTree/BP_GameTree.BP_GameTree_C" self (`self.RulesDelegate`) null (make `/Game/Manhattan/AI/GameTree/SGameTreeNode` (struct :`Type` "NewEnumerator0" :`From` (struct) :`To` (struct) :`With` (struct :`Player` "NewEnumerator0" :`Builder` "NewEnumerator0")) Game _moves)))
  (return _returnvalue))

(fn `MakeRulesDelegate`
  (returns (Rules :type "/Game/Manhattan/AI/GameTree/BP_RulesDelegate Object Reference"))
  (bind _returnvalue (`|SpawnActorFromClass` "/Game/Manhattan/AI/GameTree/BP_RulesDelegate.BP_RulesDelegate_C" (`KismetMathLibrary.MakeTransform` (0.0 0.0 0.0)) "Undefined" "OverrideRootScale" self null))
  (return _returnvalue))

(fn `RobustChild`
  (params (Tree :type "/Game/Manhattan/AI/GameTree/BP_GameTree Object Reference"))
  (returns (Child :type "/Game/Manhattan/AI/GameTree/BP_GameTree Object Reference"))
  (locals (CurrentChild :type "/Game/Manhattan/AI/GameTree/BP_GameTree Object Reference") (BestValue :type "Float (double-precision)"))
  (bind _maxs (`self.Maxs`))
  (bind _values (`BlueprintMapLibrary.Map_Values` (`/Game/Manhattan/AI/GameTree/BP_GameTree.Children` Tree)))
  (for _array_element _values
    (bind _output_get (set `local.CurrentChild` _array_element))
    (bind (_node_move _node_state _node_untriedmoves _node_visits) (break `/Game/Manhattan/AI/GameTree/SGameTreeNode` (`/Game/Manhattan/AI/GameTree/BP_GameTree.Node` _output_get)))
    (bind _returnvalue (`KismetMathLibrary.Conv_IntToDouble` _node_visits))
    (if (== _returnvalue (`local.BestValue`))
      (`KismetArrayLibrary.Array_Add` (`self.Maxs`) (`local.CurrentChild`))
      (elif (> _returnvalue (`local.BestValue`))
        (set `local.BestValue` _returnvalue)
        (set `self.Maxs` (`|MakeArray` (`local.CurrentChild`))))))
  (return (`|GetArrayItem` _maxs (`KismetMathLibrary.RandomIntegerInRange` 0 (`KismetArrayLibrary.Array_LastIndex` _maxs)))))

(fn `UserConstructionScript`)