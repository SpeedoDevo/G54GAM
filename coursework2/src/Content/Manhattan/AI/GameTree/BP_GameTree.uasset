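; BP_GameTree is a game-tree node for Monte Carlo tree search in the Manhattan AI, holding state, move, untried moves, visits and reward.
; Expansion picks a random untried move, applies it through Rules and stores the new child by move.
; Backup walks parent links to the root, adding visits and summing reward.
; BackupMonteCarlo instead calls MonteCarloReward to keep rewards in [0, 1], but that function's running-average expression is unconnected.
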(fn `Backup`
  (params (Reward :type "Vector Structure"))
  (locals (CurrentTree :type "/Game/Manhattan/AI/GameTree/BP_GameTree Object Reference"))
  (set `local.CurrentTree` self)
  (bind _currenttree (`local.CurrentTree` :!label _label)
    (:`then`
      (bind (_node_move _node_state _node_untriedmoves _node_visits _node_reward) (break `/Game/Manhattan/AI/GameTree/SGameTreeNode` (`/Game/Manhattan/AI/GameTree/BP_GameTree.Node` _currenttree)))
      ;[1 1 1] add a visit and add the computed reward
      (set `/Game/Manhattan/AI/GameTree/BP_GameTree.Node` (make `/Game/Manhattan/AI/GameTree/SGameTreeNode` _node_move _node_state _node_untriedmoves (+ _node_visits 1) (+ _node_reward Reward)) (`local.CurrentTree`))
      (set `local.CurrentTree` (`/Game/Manhattan/AI/GameTree/BP_GameTree.Parent` (`local.CurrentTree`))) ; if parent is invalid then this was the root and the loop terminates
      (goto _label))
    (:`else`
      (return))))

(fn `BackupMonteCarlo`
  (params (Reward :type "Vector Structure"))
  (locals (CurrentTree :type "/Game/Manhattan/AI/GameTree/BP_GameTree Object Reference"))
  (set `local.CurrentTree` self)
  (bind _currenttree (`local.CurrentTree` :!label _label)
    (:`then`
      (bind (_node_move _node_state _node_untriedmoves _node_visits _node_reward) (break `/Game/Manhattan/AI/GameTree/SGameTreeNode` (`/Game/Manhattan/AI/GameTree/BP_GameTree.Node` _currenttree)))
      (bind _returnvalue (`KismetMathLibrary.Conv_IntToDouble` _node_visits))
      ;[1 1 1] add a visit and add the computed reward
      (set `/Game/Manhattan/AI/GameTree/BP_GameTree.Node` (make `/Game/Manhattan/AI/GameTree/SGameTreeNode` _node_move _node_state _node_untriedmoves (+ _node_visits 1) (+ (* _node_reward (/ (- _returnvalue 1.0) _returnvalue)) (* Reward (/ 1.0 _returnvalue)))) (`local.CurrentTree`))
      (set `local.CurrentTree` (`/Game/Manhattan/AI/GameTree/BP_GameTree.Parent` (`local.CurrentTree`)))
      (goto _label))
    (:`else`
      (return))))

(fn `ChooseUntriedMove`
  (returns (Move :type "/Game/Manhattan/Core/Data/SMove Structure"))
  (bind (_node_move _node_state _node_untriedmoves) (break `/Game/Manhattan/AI/GameTree/SGameTreeNode` (`self.Node`)))
  (return (`|GetArrayItem` _node_untriedmoves (`KismetMathLibrary.RandomIntegerInRange` 0 (`KismetArrayLibrary.Array_LastIndex` _node_untriedmoves)))))

(fn `Expand`
  (returns (Child :type "/Game/Manhattan/AI/GameTree/BP_GameTree Object Reference"))
  (bind _move (`self.ChooseUntriedMove`))
  (bind _child (`self.ExpandWithMove` _move))
  (return _child))

(fn `ExpandWithMove`
  (params (Move :type "/Game/Manhattan/Core/Data/SMove Structure (by ref)"))
  (returns (Child :type "/Game/Manhattan/AI/GameTree/BP_GameTree Object Reference"))
  (bind (_node_move _node_state _node_untriedmoves) (break `/Game/Manhattan/AI/GameTree/SGameTreeNode` (`self.Node`)))
  (bind _rules (`self.Rules`))
  (`KismetArrayLibrary.Array_RemoveItem` _node_untriedmoves Move) ; make sure we don't do this move again
  ;[1 1 1] create a new node for the game state
  (bind _newgame (`/Game/Manhattan/AI/GameTree/BP_RulesDelegate.ApplyMove` _rules _node_state Move))
  (bind _moves (`/Game/Manhattan/AI/GameTree/BP_RulesDelegate.GetPossibleMoves` _rules _newgame))
  (bind _returnvalue (`|GenericCreateObject` "BP_GameTree_C" self _rules self (make `/Game/Manhattan/AI/GameTree/SGameTreeNode` (`local.Move`) _newgame _moves)))
  (`BlueprintMapLibrary.Map_Add` (`self.Children`) (`local.Move`) _returnvalue)
  (return _returnvalue))

(fn `IsFullyExpanded`
  (returns (bFullyExpanded :type Boolean))
  (bind (_node_move _node_state _node_untriedmoves) (break `/Game/Manhattan/AI/GameTree/SGameTreeNode` (`self.Node`)))
  (return (<= (`KismetArrayLibrary.Array_Length` _node_untriedmoves) 0)))

(fn `IsTerminal`
  (returns (bTerminal :type Boolean))
  (return (`|EnumEquality` (break `/Game/Manhattan/Core/Data/SGameState` (`.State_6_5E4ECDEC4B9B8149DDE0E79B934AB2CB` (break `/Game/Manhattan/AI/GameTree/SGameTreeNode` (`self.Node`)))) "NewEnumerator3")))

(fn `Split`
  (returns (Rules :type "/Game/Manhattan/AI/GameTree/BP_RulesDelegate Object Reference") (Parent :type "/Game/Manhattan/AI/GameTree/BP_GameTree Object Reference") (Children :type "Map of /Game/Manhattan/Core/Data/SMove Structure to /Game/Manhattan/AI/GameTree/BP_GameTree Object Reference") (Node :type "/Game/Manhattan/AI/GameTree/SGameTreeNode Structure"))
  (return (`self.Rules`) (`self.Parent`) (`self.Children`) (`self.Node`)))