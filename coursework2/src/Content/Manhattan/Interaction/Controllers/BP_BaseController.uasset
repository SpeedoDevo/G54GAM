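; BP_BaseController is a base controller for one player in the Manhattan board game, bound to that player from its setup on BeginPlay.
; A move request fetches possible moves from the board's display state, keeps the associated player's, and passes them to OnChooseMove.
; That function and the turn, click, undo, opponent-move and game-end events are empty hooks.
; Helpers check whose turn it is and send ticker and winner announcements to the HUD.
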(event `self.ReceiveBeginPlay`
  (bind _setup_player (break `/Game/Manhattan/Core/Engine/Game/SControllerSetup` (`self.Setup`)))
  (set `self.AssociatedPlayer` _setup_player))

(event `OnRequestMove`
  (bind _moves (`/Game/Manhattan/Core/Rules/BPFL_Rules.GetPossibleMoves` (`/Game/Manhattan/Interaction/Board/BP_Board.DisplayState` (`/Game/Manhattan/Core/Util/BPFL_Util.GetBoard`))))
  (bind _moves_2 (`self.FilterMovesToAssociatedPlayer` _moves))
  (`self.OnChooseMove` _moves_2))

(event `OnStartTurn`)

(event `OnMoveClicked`
  (params (Move :type "/Game/Manhattan/Core/Data/SMove Structure")))

(event `OnBuilderClicked`
  (params (Indicator :type "/Game/Manhattan/Interaction/SelectionIndicator/BP_SelectionIndicator Object Reference")))

(event `OnEndTurn`)

(event `OnUndo`)

(event `OnFinishGame`)

(event `OnOpponentMove`
  (params (Move :type "/Game/Manhattan/Core/Data/SMove Structure")))

(fn `AnnounceTicker`
  (params (Text :type String))
  (`/Game/Manhattan/Interaction/HUD/BP_HUDWidget.OnTickerAnnouncement` (`/Game/Manhattan/Core/Util/BPFL_Util.GetHUD`) Text)
  (return))

(fn `AnnounceWinner`
  (params (Text :type String))
  (`/Game/Manhattan/Interaction/HUD/BP_HUDWidget.OnWinnerAnnouncement` (`/Game/Manhattan/Core/Util/BPFL_Util.GetHUD`) Text)
  (return))

(fn `FilterMovesToAssociatedPlayer`
  (params (InMoves :type "Array of /Game/Manhattan/Core/Data/SMove Structure (by ref)"))
  (returns (Moves :type "Array of /Game/Manhattan/Core/Data/SMove Structure"))
  (locals (OutMoves :type "Array of /Game/Manhattan/Core/Data/SMove Structure") (Move :type "/Game/Manhattan/Core/Data/SMove Structure"))
  (for _array_element InMoves
    (bind _output_get (set `local.Move` _array_element))
    (if (== (`self.AssociatedPlayer`) (break `/Game/Manhattan/Core/Data/SBuilder` (`.With_20_14AF0B304C5F797DFB975AB7C5998B26` (break `/Game/Manhattan/Core/Data/SMove` _output_get))))
      (`KismetArrayLibrary.Array_Add` (`local.OutMoves`) (`local.Move`))))
  (return (`local.OutMoves`)))

(fn `IsTakingControl`
  (returns (Controlling :type Boolean))
  (bind (_gamestate_phase _gamestate_board _gamestate_currentplayer) (break `/Game/Manhattan/Core/Data/SGameState` (`/Game/Manhattan/Core/Util/BPFL_Util.GetSGameState`)))
  (return (== (`self.AssociatedPlayer`) _gamestate_currentplayer)))

(fn `OnChooseMove`
  (params (Moves :type "Array of /Game/Manhattan/Core/Data/SMove Structure")))

(fn `UserConstructionScript`)