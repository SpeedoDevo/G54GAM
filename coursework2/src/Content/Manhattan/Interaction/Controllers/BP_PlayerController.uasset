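; Player controller for the Manhattan board game that runs a human turn, from HUD announcement through choosing, undoing and committing moves.
; Spawns clickable move indicators on the board, filtered in the MOVE phase by the selected builder, which is auto-selected when only one can move.
; Clicked moves update a local display state and buffer until end turn commits them to the game state.
; Undo drops the last move and replays the rest.
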(event `self.OnStartTurn`
  (bind _hud (`/Game/Manhattan/Core/Util/BPFL_Util.GetHUD`))
  (bind (_setup_player _setup_type _setup_difficulty _setup_name) (break `/Game/Manhattan/Core/Engine/Game/SControllerSetup` (`self.Setup`)))
  ;[1 1 1] turn start, announce to player, enable buttons
  (`self.AnnounceTicker` (`KismetStringLibrary.Concat_StrStr` "Your turn " _setup_name))
  (`/Game/Manhattan/Interaction/HUD/BP_HUDWidget.OnSetButtonsEnabled` _hud true)
  (`/Game/Manhattan/Interaction/HUD/BP_HUDWidget.OnSetButtonsVisible` _hud true))

(event `self.OnChooseMove`
  (params (Moves :type "Array of /Game/Manhattan/Core/Data/SMove Structure (by ref)"))
  ;[1 1 1] choose a move by rendering the indicators on the board
  (set `self.PossibleMoves` Moves)
  (set `self.DisplayState` (`/Game/Manhattan/Interaction/Board/BP_Board.DisplayState` (`/Game/Manhattan/Core/Util/BPFL_Util.GetBoard`)))
  (`self.OnRenderMoves`))

(event `self.OnMoveClicked`
  (params (Move :type "/Game/Manhattan/Core/Data/SMove Structure"))
  ;[1 1 1] when a move is clicked then add it to the move buffer, and render the new state
  (bind _newgame (`/Game/Manhattan/Core/Rules/BPFL_Rules.ApplyMove` (`self.DisplayState`) Move))
  (set `self.DisplayState` _newgame)
  (`KismetArrayLibrary.Array_Add` (`self.UncommitedMoves`) Move)
  (`self.ClearIndicators` true)
  (`/Game/Manhattan/Interaction/Board/BP_Board.OnRenderState` (`/Game/Manhattan/Core/Util/BPFL_Util.GetBoard`) (`self.DisplayState`)))

(event `self.OnBuilderClicked`
  (params (Indicator :type "/Game/Manhattan/Interaction/SelectionIndicator/BP_SelectionIndicator Object Reference"))
  ;[1 1 1] when a builder is clicked update the selection and render moves
  (`self.UpdateSelection` Indicator)
  (`self.ClearIndicators` false)
  (`self.OnRenderMoves`) ; no render state as the game state hasn't changed
)

(event `OnRenderMoves`
  (bind _possiblemoves (`self.PossibleMoves`))
  ;[1 1 1] show all indicators given the available moves
  (`self.UpdateButtons`)
  (`self.ShowSelection` _possiblemoves)
  (bind _moves (`self.FilterMovesToSelection` _possiblemoves))
  (for _array_element _moves
    (bind _returnvalue (`|SpawnActorFromClass` "/Game/Manhattan/Interaction/MoveIndicator/BP_MoveIndicator.BP_MoveIndicator_C" (`KismetMathLibrary.MakeTransform` (`/Game/Manhattan/Interaction/Board/BP_Board.FindAttachmentLocation` (`/Game/Manhattan/Core/Util/BPFL_Util.GetBoard`) (`.To_19_32569A5F497DE1A38335F7B25B4D56CA` (break `/Game/Manhattan/Core/Data/SMove` _array_element)))) "Undefined" "OverrideRootScale" null _array_element null))
    (`KismetArrayLibrary.Array_Add` (`self.MoveIndicators`) _returnvalue)))

(event `self.OnEndTurn`
  ;[1 1 1] end turn, clean up indicators and commit moves
  (`self.ClearIndicators` true)
  (`BlueprintSetLibrary.Set_Clear` (`self.SelectedBuilder`))
  (`/Game/Manhattan/Interaction/HUD/BP_HUDWidget.OnSetButtonsEnabled` (`/Game/Manhattan/Core/Util/BPFL_Util.GetHUD`) false)
  (bind _gamestate (`/Game/Manhattan/Core/Engine/Game/BP_ManhattanGameState.CommitMoves` (`/Game/Manhattan/Core/Util/BPFL_Util.GetManhattanGameState`) (`self.UncommitedMoves`)))
  (`KismetArrayLibrary.Array_Clear` (`self.UncommitedMoves`))
  (bind _output_get (set `self.DisplayState` _gamestate))
  (`/Game/Manhattan/Interaction/Board/BP_Board.OnRenderState` (`/Game/Manhattan/Core/Util/BPFL_Util.GetBoard`) _output_get))

(event `self.OnUndo`
  (bind _uncommitedmoves (`self.UncommitedMoves`))
  ;[1 1 1] undo: pop the last move from the undo buffer, refresh the game state and render it
  (`KismetArrayLibrary.Array_RemoveItem` _uncommitedmoves (`|GetArrayItem` _uncommitedmoves (`KismetArrayLibrary.Array_LastIndex` _uncommitedmoves)))
  (set `self.DisplayState` (`/Game/Manhattan/Core/Util/BPFL_Util.GetSGameState`))
  (for _array_element (`self.UncommitedMoves`)
    (bind _newgame (`/Game/Manhattan/Core/Rules/BPFL_Rules.ApplyMove` (`self.DisplayState`) _array_element))
    (set `self.DisplayState` _newgame))
  (set `self.bGameFinished` false)
  (`self.ClearIndicators` true)
  (`/Game/Manhattan/Interaction/Board/BP_Board.OnRenderState` (`/Game/Manhattan/Core/Util/BPFL_Util.GetBoard`) (`self.DisplayState`)))

(event `self.OnFinishGame`
  ;[1 1 1] finish game
  (set `self.bGameFinished` true)
  (`self.UpdateButtons`))

(fn `ClearIndicators`
  (params (bClearSelection :type Boolean))
  (`|ExecutionSequence`
    (:`then_0`
      (for _array_element (`self.MoveIndicators`)
        (`self.K2_DestroyActor` _array_element))
      (`KismetArrayLibrary.Array_Clear` (`self.MoveIndicators`)))
    (:`then_1`
      (if bClearSelection
        (for _array_element_2 (`self.SelectionIndicators`)
          (`self.K2_DestroyActor` _array_element_2))
        (`KismetArrayLibrary.Array_Clear` (`self.SelectionIndicators`))))
    (:`then_2`
      (return))))

(fn `FilterMovesToSelection`
  (params (InMoves :type "Array of /Game/Manhattan/Core/Data/SMove Structure (by ref)"))
  (returns (Moves :type "Array of /Game/Manhattan/Core/Data/SMove Structure"))
  (locals (OutMoves :type "Array of /Game/Manhattan/Core/Data/SMove Structure") (Move :type "/Game/Manhattan/Core/Data/SMove Structure"))
  (bind _displaystate_phase (break `/Game/Manhattan/Core/Data/SGameState` (`self.DisplayState`)))
  (switch `/Game/Manhattan/Core/Data/EGamePhase` _displaystate_phase
    (:`NewEnumerator0`
      _)
    (:`NewEnumerator1`
      (set `local.OutMoves` (`|MakeArray`))
      (for _array_element (`local.InMoves`)
        (bind _output_get (set `local.Move` _array_element))
        (if (`BlueprintSetLibrary.Set_Contains` (`self.SelectedBuilder`) (`.With_20_14AF0B304C5F797DFB975AB7C5998B26` (break `/Game/Manhattan/Core/Data/SMove` _output_get)))
          (`KismetArrayLibrary.Array_Add` (`local.OutMoves`) (`local.Move`))))
      (return (`local.OutMoves`)))
    (:`NewEnumerator2`
      _)
    (:`NewEnumerator3`
      _))
  (return InMoves) ; only applies to MOVE moves\ndo nothing
)

(fn `ShowSelection`
  (params (InMoves :type "Array of /Game/Manhattan/Core/Data/SMove Structure"))
  (locals (Move :type "/Game/Manhattan/Core/Data/SMove Structure") (BuildersWithIndicators :type "Set of /Game/Manhattan/Core/Data/SBuilder Structure"))
  (bind (_move_type _move_from _move_to _move_with) (break `/Game/Manhattan/Core/Data/SMove` (`local.Move`)))
  (bind (_move_type_2 _move_from_2 _move_to_2 _move_with_2) (break `/Game/Manhattan/Core/Data/SMove` (`local.Move`)))
  (bind _returnvalue (`BlueprintSetLibrary.Set_Contains` (`self.SelectedBuilder`) _move_with_2))
  (bind _output (`|GetArrayItem` (`self.SelectionIndicators`)))
  (if (<= (`KismetArrayLibrary.Array_Length` (`self.SelectionIndicators`)) 0)
    (for _array_element InMoves
      (bind _output_get (set `local.Move` _array_element))
      (switch `/Game/Manhattan/Core/Data/EMoveType` (break `/Game/Manhattan/Core/Data/SMove` _output_get) ; for each MOVE move
        (:`NewEnumerator1`
          (if (not (`BlueprintSetLibrary.Set_Contains` (`local.BuildersWithIndicators`) (`.With_20_14AF0B304C5F797DFB975AB7C5998B26` (break `/Game/Manhattan/Core/Data/SMove` _output_get))))
            (bind _returnvalue_2 (`|SpawnActorFromClass` "/Game/Manhattan/Interaction/SelectionIndicator/BP_SelectionIndicator.BP_SelectionIndicator_C" (`KismetMathLibrary.MakeTransform` (`/Game/Manhattan/Interaction/Board/BP_Board.FindAttachmentLocation` (`/Game/Manhattan/Core/Util/BPFL_Util.GetBoard`) _move_from_2)) "Undefined" "OverrideRootScale" null _move_with_2 _returnvalue null)) ; create an indicator
            (`KismetArrayLibrary.Array_Add` (`self.SelectionIndicators`) _returnvalue_2)
            (`BlueprintSetLibrary.Set_Add` (`local.BuildersWithIndicators`) _move_with)
            (if _returnvalue
              (set `self.ActiveSelectionIndicator` _returnvalue_2)))))))
  (if (== (`KismetArrayLibrary.Array_Length` (`self.SelectionIndicators`)) 1)
    (`self.UpdateSelection` _output) ; then automatically select it
    (`/Game/Manhattan/Interaction/SelectionIndicator/BP_SelectionIndicator.OnSelected` _output)
    (return)
    (else
      (return))))

(fn `UpdateButtons`
  (`self.UpdateUndoButton`)
  (`self.UpdateEndTurnButton`)
  (return))

(fn `UpdateEndTurnButton`
  (bind _bgamefinished (`self.bGameFinished`))
  (bind (_displaystate_phase _displaystate_board _displaystate_currentplayer) (break `/Game/Manhattan/Core/Data/SGameState` (`self.DisplayState`)))
  (`/Game/Manhattan/Interaction/HUD/BP_HUDWidget.OnSetEndTurnEnabled` (`/Game/Manhattan/Core/Util/BPFL_Util.GetHUD`) (or (!= (`self.AssociatedPlayer`) _displaystate_currentplayer) _bgamefinished) _bgamefinished)
  (return))

(fn `UpdateSelection`
  (params (Indicator :type "/Game/Manhattan/Interaction/SelectionIndicator/BP_SelectionIndicator Object Reference"))
  (bind _selectedbuilder (`self.SelectedBuilder`))
  (`BlueprintSetLibrary.Set_Clear` _selectedbuilder)
  (`BlueprintSetLibrary.Set_Add` _selectedbuilder (`/Game/Manhattan/Interaction/SelectionIndicator/BP_SelectionIndicator.Builder` Indicator))
  (bind _activeselectionindicator (`self.ActiveSelectionIndicator`)
    (:`then`
      (`/Game/Manhattan/Interaction/SelectionIndicator/BP_SelectionIndicator.OnDeselected` _activeselectionindicator))
    (:`else`
      _))
  (set `self.ActiveSelectionIndicator` Indicator))

(fn `UpdateUndoButton`
  (`/Game/Manhattan/Interaction/HUD/BP_HUDWidget.OnSetUndoEnabled` (`/Game/Manhattan/Core/Util/BPFL_Util.GetHUD`) (> (`KismetArrayLibrary.Array_Length` (`self.UncommitedMoves`)) 0))
  (return))

(fn `UserConstructionScript`)