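; AI controller for the Manhattan board game that plays a uniformly random legal move on its turn.
; At turn start it shows a ticker saying the player is thinking.
; When asked to choose, it waits for a delay, commits one random move through the Manhattan game state and passes the result to the board to render.
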(event `self.OnStartTurn`
  (bind (_setup_player _setup_type _setup_difficulty _setup_name) (break `/Game/Manhattan/Core/Engine/Game/SControllerSetup` (`self.Setup`)))
  (`self.AnnounceTicker` (`KismetStringLibrary.Concat_StrStr` _setup_name " is thinking....")))

(event `self.OnChooseMove`
  (params (Moves :type "Array of /Game/Manhattan/Core/Data/SMove Structure (by ref)"))
  (`KismetSystemLibrary.Delay` (`self.Delay`))
  (bind _gamestate (`/Game/Manhattan/Core/Engine/Game/BP_ManhattanGameState.CommitMoves` (`/Game/Manhattan/Core/Util/BPFL_Util.GetManhattanGameState`) (`|MakeArray` (`|GetArrayItem` Moves (`KismetMathLibrary.RandomIntegerInRange` 0 (`KismetArrayLibrary.Array_LastIndex` Moves))))))
  (`/Game/Manhattan/Interaction/Board/BP_Board.OnRenderState` (`/Game/Manhattan/Core/Util/BPFL_Util.GetBoard`) _gamestate))

(fn `UserConstructionScript`
  (`parent.UserConstructionScript`))