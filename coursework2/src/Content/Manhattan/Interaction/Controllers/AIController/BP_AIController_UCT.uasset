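; AI controller for the Manhattan board game that picks moves with a UCT tree search.
; On BeginPlay it spawns an optimised UCT searcher tuned by a difficulty row from a data table.
; Completed searches commit and render the move, while opponent moves advance the search tree.
; A looping timer feeds the HUD progress bar, treating each search as half of a two-move turn.
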(event `self.ReceiveBeginPlay`
  (bind (_parameters_rolloutdepth _parameters_frameratetradeoff _parameters_targetconfidence) (break `/Game/Manhattan/Interaction/Controllers/AIController/SAIDifficultySetting` (`self.GetDifficultyParameters`)))
  (bind (_setup_player _setup_type _setup_difficulty) (break `/Game/Manhattan/Core/Engine/Game/SControllerSetup` (`self.Setup`)))
  ;[1 1 1] setup the search algo
  (`parent.ReceiveBeginPlay`)
  (set `self.Difficulty` _setup_difficulty)
  (bind _returnvalue (`|SpawnActorFromClass` "/Game/Manhattan/AI/UCT/Optimised/BP_UCT_Optimised.BP_UCT_Optimised_C" (`KismetMathLibrary.MakeTransform` (0.0 0.0 0.0)) "Undefined" "OverrideRootScale" null _parameters_rolloutdepth _parameters_frameratetradeoff _parameters_targetconfidence null))
  (bind _output_get (set `self.UCT` _returnvalue))
  (add `/Game/Manhattan/AI/UCT/Base/BP_UCT.OnSearchComplete` _output_get (delegate `OnSearchComplete`)))

(event `self.OnStartTurn`
  (bind (_setup_player _setup_type _setup_difficulty _setup_name) (break `/Game/Manhattan/Core/Engine/Game/SControllerSetup` (`self.Setup`)))
  (set `self.MoveCounter` -1)
  (`self.AnnounceTicker` (`KismetStringLibrary.Concat_StrStr` _setup_name " is thinking....")) ; announce turn start to player
  (bind _returnvalue (`KismetSystemLibrary.K2_SetTimerDelegate` (delegate `OnProgress`) 0.5 true)) ; create an event to update the progress bar at 2fps
)

(event `OnProgress`
  (`/Game/Manhattan/Interaction/HUD/BP_HUDWidget.OnProgressUpdate` (`/Game/Manhattan/Core/Util/BPFL_Util.GetHUD`) (+ (/ (`/Game/Manhattan/AI/UCT/Optimised/BP_UCT_Optimised.GetProgress` (`self.UCT`)) 2.0) (select `int` (`self.MoveCounter`) :`0` 0.0 :`1` 0.5 :!type "Float (single-precision)"))))

(event `OnSearchComplete`
  (params (Move :type "/Game/Manhattan/Core/Data/SMove Structure"))
  ;[1 1 1] when found a move commit and render it
  (bind _gamestate (`/Game/Manhattan/Core/Engine/Game/BP_ManhattanGameState.CommitMoves` (`/Game/Manhattan/Core/Util/BPFL_Util.GetManhattanGameState`) (`|MakeArray` Move)))
  (`/Game/Manhattan/Interaction/Board/BP_Board.OnRenderState` (`/Game/Manhattan/Core/Util/BPFL_Util.GetBoard`) _gamestate)
  (bind (_phase _board _currentplayer) (break `/Game/Manhattan/Core/Data/SGameState` _gamestate))
  (if (or (`|EnumEquality` _phase "NewEnumerator3") (`|EnumInequality` _currentplayer (`self.AssociatedPlayer`)))
    (`KismetSystemLibrary.K2_ClearAndInvalidateTimerHandle` (stale `self.OnStartTurn` _returnvalue))
    (`/Game/Manhattan/Interaction/HUD/BP_HUDWidget.OnProgressUpdate` (`/Game/Manhattan/Core/Util/BPFL_Util.GetHUD`) 1.0)))

(event `self.OnChooseMove`
  (params (Moves :type "Array of /Game/Manhattan/Core/Data/SMove Structure (by ref)"))
  ;[1 1 1] start the search
  (`/Engine/EditorBlueprintResources/StandardMacros.IncrementInt` (`self.MoveCounter`)
    (:`  `
      (`/Game/Manhattan/AI/UCT/Base/BP_UCT.OnSearch` (`self.UCT`) (`/Game/Manhattan/Core/Util/BPFL_Util.GetSGameState`)))))

(event `self.OnOpponentMove`
  (params (Move :type "/Game/Manhattan/Core/Data/SMove Structure"))
  (`/Game/Manhattan/AI/UCT/Optimised/BP_UCT_Optimised.OnAdvanceTree` (`self.UCT`) Move))

(fn `GetDifficultyParameters`
  (returns (Parameters :type "/Game/Manhattan/Interaction/Controllers/AIController/SAIDifficultySetting Structure"))
  (bind _returnvalue (`|GetDataTableRow` "/Game/Manhattan/Interaction/Controllers/AIController/DT_AIDifficultyCurve.DT_AIDifficultyCurve" (`KismetStringLibrary.Conv_StringToName` (`|GetEnumeratorNameAsString` (`self.Difficulty`))))
    (:`then`
      (return _returnvalue))
    (:`RowNotFound`
      (`/Game/Manhattan/Core/Rules/BPFL_Rules.ShowError` "AIController" "difficulty parameters not found")
      (return))))

(fn `UserConstructionScript`)