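; BP_CharacterPool keeps hidden, pre-spawned builders and height-keyed blocks for displaying moves on the board.
; BeginPlay creates one actor per builder type and per block height, stored in maps.
; Show and Hide resolve a move to an actor and attachment location: builders for setup or move, next-height block for build; hiding requires the actor still be there.
; ConsumeBlock hands out a visible block and spawns its replacement.
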(event `self.ReceiveBeginPlay`
  (for _array_element (`|MakeArray` (make `/Game/Manhattan/Core/Data/SBuilder` "NewEnumerator0") (make `/Game/Manhattan/Core/Data/SBuilder` "NewEnumerator0" "NewEnumerator1") (make `/Game/Manhattan/Core/Data/SBuilder` "NewEnumerator1") (make `/Game/Manhattan/Core/Data/SBuilder` "NewEnumerator1" "NewEnumerator1"))
    (`self.CreateBuilder` _array_element))
  (for _index (range 1 5)
    (`self.CreateBlock` _index)))

(fn `ConsumeBlock`
  (params (Height :type "Integer (by ref)"))
  (returns (Block :type "/Game/Manhattan/Characters/BP_SmartBlock Object Reference"))
  (locals (OutBlock :type "/Game/Manhattan/Characters/BP_SmartBlock Object Reference"))
  (bind _outblock (`local.OutBlock`))
  (set `local.OutBlock` (`BlueprintMapLibrary.Map_Find` (`self.Blocks`) Height))
  (`self.CreateBlock` (`local.Height`)) ; create a block that will\nreplace this one
  (`self.SetActorHiddenInGame` _outblock false)
  (return _outblock))

(fn `CreateBlock`
  (params (Height :type Integer))
  (bind _returnvalue (`|SpawnActorFromClass` "/Game/Manhattan/Characters/BP_SmartBlock.BP_SmartBlock_C" (`KismetMathLibrary.MakeTransform` (0.0 0.0 0.0)) "Undefined" "OverrideRootScale" null Height null))
  (`BlueprintMapLibrary.Map_Add` (`self.Blocks`) Height _returnvalue)
  (`self.SetActorHiddenInGame` _returnvalue true))

(fn `CreateBuilder`
  (params (Builder :type "/Game/Manhattan/Core/Data/SBuilder Structure"))
  (bind _returnvalue (`|SpawnActorFromClass` "/Game/Manhattan/Characters/BP_Builder.BP_Builder_C" (`KismetMathLibrary.MakeTransform` (0.0 0.0 0.0)) "Undefined" "OverrideRootScale" null Builder null))
  (`BlueprintMapLibrary.Map_Add` (`self.Builders`) Builder _returnvalue)
  (`self.SetActorHiddenInGame` _returnvalue true))

(fn `FindActorAndLocationForMove`
  (params (Move :type "/Game/Manhattan/Core/Data/SMove Structure (by ref)"))
  (returns (Actor :type "Actor Object Reference") (Location :type "Vector Structure"))
  (bind _location (`/Game/Manhattan/Interaction/Board/BP_Board.FindAttachmentLocation` (`/Game/Manhattan/Core/Util/BPFL_Util.GetBoard`) Move_To_19_32569A5F497DE1A38335F7B25B4D56CA))
  (bind (_position_id _position_height) (break `/Game/Manhattan/Core/Data/sBoardPosition` (`/Game/Manhattan/Core/Rules/BPFL_Rules.GetPositionFromId` (`/Game/Manhattan/Interaction/Board/BP_Board.DisplayState` (`/Game/Manhattan/Core/Util/BPFL_Util.GetBoard`)) Move_To_19_32569A5F497DE1A38335F7B25B4D56CA)))
  (switch `/Game/Manhattan/Core/Data/EMoveType` Move_Type_15_6A7ECA5746BCEAC1E8884D97A17345E5
    (:`NewEnumerator0`
      _)
    (:`NewEnumerator1`
      _)
    (:`NewEnumerator2`
      (return (`BlueprintMapLibrary.Map_Find` (`self.Blocks`) (+ _position_height 1)) _location) ; on build display a block
    ))
  (return (`BlueprintMapLibrary.Map_Find` (`self.Builders`) Move_With_20_14AF0B304C5F797DFB975AB7C5998B26) _location) ; on move or setup display a builder
)

(fn `HideActorForMove`
  (params (Move :type "/Game/Manhattan/Core/Data/SMove Structure (by ref)"))
  (bind (_actor _location) (`self.FindActorAndLocationForMove` Move))
  (if (== (`self.K2_GetActorLocation` _actor) _location :`ErrorTolerance` 1.0)
    (`self.SetActorHiddenInGame` _actor true))
  (return))

(fn `ShowActorForMove`
  (params (Move :type "/Game/Manhattan/Core/Data/SMove Structure (by ref)"))
  (bind (_actor _location) (`self.FindActorAndLocationForMove` Move))
  (`self.K2_SetActorLocation` _actor _location false true)
  (`self.SetActorHiddenInGame` _actor false)
  (return))

(fn `UserConstructionScript`)