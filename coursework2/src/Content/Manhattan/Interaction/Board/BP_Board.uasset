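; BP_Board is the Manhattan game board actor that renders game states, rotates the camera on right-click drag and announces the winner.
; OnRenderState reconciles each position with the state, adding or removing blocks and builders, then fires a phase-dependent controller event through a gate closed at game end.
; Blocks come from the character pool and stack via a per-position attachment map, seeded with a construction-script grid of arrow components and updated to each top block.
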(event `self.ReceiveBeginPlay`
  ;[1 1 1] initialise board state from the global game state
  (`/Game/Manhattan/Core/Util/BPFL_Util.FireEventOnCurrentController` "NewEnumerator5")
  (`self.OnRenderState` (`/Game/Manhattan/Core/Util/BPFL_Util.GetSGameState`)))

(event `InputAxis|CameraTurn`
  (params (AxisValue :type "Float (single-precision)"))
  ;[1 1 1] handle mouse input
  (if (`self.bCameraTurning`)
    (`SceneComponent.K2_AddLocalRotation` (`self.CameraRotator`) (`KismetMathLibrary.MakeRotator` 0.0 0.0 (* (`self.GetInputAxisValue`) 5.0)) false false)))

(event `InputAction|RightClick` :consume false
  (params (Key :type "Key Structure"))
  ;[1 1 1] handle mouse input
  (:`Pressed`
    (set `self.bCameraTurning` true))
  (:`Released`
    (set `self.bCameraTurning` false)))

(event `OnRenderState`
  (params (DisplayState :type "/Game/Manhattan/Core/Data/SGameState Structure"))
  ;[1 1 1] show a given board state and fire the consequent events
  (bind _output_get (set `self.DisplayState` DisplayState))
  (`self.ShowCharacters`)
  (`/Engine/EditorBlueprintResources/StandardMacros.Gate` false :!label _label
    (:`Exit`
      (if (`|EnumEquality` (break `/Game/Manhattan/Core/Data/SGameState` _output_get) "NewEnumerator3")
        (`/Game/Manhattan/Core/Util/BPFL_Util.FireEventOnCurrentController` "NewEnumerator6")
        (else
          (`/Game/Manhattan/Core/Util/BPFL_Util.FireEventOnCurrentController` "NewEnumerator0"))))))

(event `OnFinished`
  (bind (_gamestate_phase _gamestate_board _gamestate_currentplayer _gamestate_movedbuilder _gamestate_setupcounter _gamestate_winningplayer) (break `/Game/Manhattan/Core/Data/SGameState` (`/Game/Manhattan/Core/Util/BPFL_Util.GetSGameState`)))
  (bind (_output_player _output_type _output_difficulty _output_name) (break `/Game/Manhattan/Core/Engine/Game/SControllerSetup` (`/Game/Manhattan/Core/Engine/Game/BP_ManhattanGameInstance.GetPlayerControllerSetup` (`/Game/Manhattan/Core/Util/BPFL_Util.GetManhattanGameInstance`) _gamestate_winningplayer)))
  ;[1 1 1] handle end game
  (`/Game/Manhattan/Interaction/HUD/BP_HUDWidget.OnWinnerAnnouncement` (`/Game/Manhattan/Core/Util/BPFL_Util.GetHUD`) (`KismetStringLibrary.Concat_StrStr` _output_name " wins"))
  (`|ExecutionSequence`
    (:`then_0`
      (goto _label :!via `Close`))
    (:`then_1`
      (`self.OnRenderState` (`/Game/Manhattan/Core/Util/BPFL_Util.GetSGameState`)))
    (:`then_2`
      (`/Game/Manhattan/Interaction/HUD/BP_HUDWidget.OnSetButtonsVisible` (`/Game/Manhattan/Core/Util/BPFL_Util.GetHUD`) false))))

(fn `AddActorToBlocks`
  (params (Position :type "/Game/Manhattan/Core/Data/SBoardPositionId Structure (by ref)") (InActor :type "Actor Object Reference (by ref)"))
  (locals (BlocksInPosition :type "Array of Actor Object Reference"))
  (bind (_value _returnvalue) (`BlueprintMapLibrary.Map_Find` (`self.Blocks`) Position))
  (bind _returnvalue_actors (break `/Game/Manhattan/Core/Util/SActorArray` (select `bool` _returnvalue :`false` (make `/Game/Manhattan/Core/Util/SActorArray` (`|MakeArray`)) :`true` _value)))
  (bind _output_get (set `local.BlocksInPosition` _returnvalue_actors))
  (`KismetArrayLibrary.Array_Add` _output_get (`local.InActor`)) ; add the actor
  (`BlueprintMapLibrary.Map_Add` (`self.Blocks`) (`local.Position`) (make `/Game/Manhattan/Core/Util/SActorArray` (`local.BlocksInPosition`)))
  (return))

(fn `FindAttachmentLocation`
  (params (Position :type "/Game/Manhattan/Core/Data/SBoardPositionId Structure (by ref)"))
  (returns (Location :type "Vector Structure"))
  (return (`SceneComponent.K2_GetComponentLocation` (`BlueprintMapLibrary.Map_Find` (`self.AttachmentMap`) Position))))

(fn `PlaceBlockFromCharacterPool`
  (params (Amount :type Integer) (Position :type "/Game/Manhattan/Core/Data/sBoardPosition Structure"))
  (locals (PositionId :type "/Game/Manhattan/Core/Data/SBoardPositionId Structure"))
  (set `local.PositionId` Position_Id_24_017E124C4617FE97DF27A688894F59A4)
  (for _index (range (+ (- Position_Height_20_CD1CD47C4EB2FF32DE9AD6A7272861B4 Amount) 1) (+ Position_Height_20_CD1CD47C4EB2FF32DE9AD6A7272861B4 1))
    (bind _block (`/Game/Manhattan/Interaction/CharacterPool/BP_CharacterPool.ConsumeBlock` (`/Game/Manhattan/Core/Util/BPFL_Util.GetCharacterPool`) _index))
    (`self.K2_SetActorLocation` _block (`self.FindAttachmentLocation` (`local.PositionId`)) false false)
    (`self.RegisterBlock` (`local.PositionId`) _block)))

(fn `RegisterBlock`
  (params (Position :type "/Game/Manhattan/Core/Data/SBoardPositionId Structure (by ref)") (Block :type "/Game/Manhattan/Characters/BP_SmartBlock Object Reference (by ref)"))
  (bind _block (`local.Block`))
  (if (`/Game/Manhattan/Characters/BP_SmartBlock.bHasAttachment` Block)
    (`self.AddActorToBlocks` (`local.Position`) _block)
    (`BlueprintMapLibrary.Map_Add` (`self.AttachmentMap`) (`local.Position`) (`/Game/Manhattan/Characters/BP_SmartBlock.Attachment` _block))
    (else
      (`self.AddActorToBlocks` (`local.Position`) (`local.Block`))
      (`BlueprintMapLibrary.Map_Remove` (`self.AttachmentMap`) (`local.Position`)))))

(fn `RemoveBlocks`
  (params (Amount :type Integer) (Position :type "/Game/Manhattan/Core/Data/sBoardPosition Structure (by ref)"))
  (locals (PositionId :type "/Game/Manhattan/Core/Data/SBoardPositionId Structure") (ActorArray :type "Array of Actor Object Reference"))
  (bind _actorarray (`local.ActorArray`))
  (set `local.PositionId` Position_Id_24_017E124C4617FE97DF27A688894F59A4)
  (for _ (range Amount)
    ;[1 1 1] find the block on the top, destroy it
    (bind _output_get (set `local.ActorArray` (break `/Game/Manhattan/Core/Util/SActorArray` (`BlueprintMapLibrary.Map_Find` (`self.Blocks`) (`local.PositionId`)))))
    (bind _returnvalue (`KismetArrayLibrary.Array_LastIndex` _output_get))
    (`self.K2_DestroyActor` (`|GetArrayItem` _output_get _returnvalue))
    (`KismetArrayLibrary.Array_Remove` (`local.ActorArray`) _returnvalue)
    (`BlueprintMapLibrary.Map_Add` (`self.Blocks`) (`local.PositionId`) (make `/Game/Manhattan/Core/Util/SActorArray` (`local.ActorArray`)))
    (if (<= (`KismetArrayLibrary.Array_Length` (`local.ActorArray`)) 0)
      ;[1 1 1] reset the attachment to the base of the board
      (`BlueprintMapLibrary.Map_Add` (`self.AttachmentMap`) (`local.PositionId`) (`BlueprintMapLibrary.Map_Find` (`self.BaseAttachmentMap`) (`local.PositionId`)))
      (else
        ;[1 1 1] find the block that is on the top after, and put its attachment point in the map
        (bind _asbp_smart_block (cast `/Game/Manhattan/Characters/BP_SmartBlock` (`|GetArrayItem` _actorarray (`KismetArrayLibrary.Array_LastIndex` _actorarray))))
        (bind _attachment (`/Game/Manhattan/Characters/BP_SmartBlock.Attachment` _asbp_smart_block))
        (`/Engine/EditorBlueprintResources/StandardMacros.IsValid` _attachment
          (:`Is Valid`
            (`BlueprintMapLibrary.Map_Add` (`self.AttachmentMap`) (`local.PositionId`) _attachment))
          (:`Is Not Valid`
            (`/Game/Manhattan/Core/Rules/BPFL_Rules.ShowError` "remove block" "removed something from above a top block?") ; the block should have an attachment point that's what\nthe previous branch was checking for
          )))))
  (return))

(fn `ShowBlocks`
  (params (Position :type "/Game/Manhattan/Core/Data/sBoardPosition Structure (by ref)"))
  (locals (PositionId :type "/Game/Manhattan/Core/Data/SBoardPositionId Structure") (PreviewActor :type "Actor Object Reference") (ModelViewDiff :type Integer :default 0))
  (set `local.PositionId` Position_Id_24_017E124C4617FE97DF27A688894F59A4)
  ;[1 1 1] find the difference between the number of blocks in the world vs the number required
  (bind _output_get (set `local.ModelViewDiff` (- Position_Height_20_CD1CD47C4EB2FF32DE9AD6A7272861B4 (`KismetArrayLibrary.Array_Length` (break `/Game/Manhattan/Core/Util/SActorArray` (`BlueprintMapLibrary.Map_Find` (`self.Blocks`) (`local.PositionId`)))))))
  (switch `int` (`KismetMathLibrary.SignOfInteger` _output_get) ; if the diff is positive then add otherwise remove
    (:`-1`
      (`self.RemoveBlocks` (`KismetMathLibrary.Abs_Int` (`local.ModelViewDiff`)) (`local.Position`))
      (return))
    (:`0`
      (return))
    (:`1`
      (`self.PlaceBlockFromCharacterPool` (`local.ModelViewDiff`) (`local.Position`)))))

(fn `ShowBuilders`
  (params (Position :type "/Game/Manhattan/Core/Data/sBoardPosition Structure (by ref)"))
  (locals (PositionId :type "/Game/Manhattan/Core/Data/SBoardPositionId Structure"))
  (bind _boccupied (`/Game/Manhattan/Core/Rules/BPFL_Rules.IsPositionOccupied` (`local.Position`)))
  ;[1 1 1] see if there is a difference between model and view
  (bind _output_get (set `local.PositionId` Position_Id_24_017E124C4617FE97DF27A688894F59A4))
  (if (!= (`.ReturnValue` (`BlueprintMapLibrary.Map_Find` (`self.Builders`) _output_get)) _boccupied)
    (if _boccupied
      ;[1 1 1] create the actor and add it to the map
      (bind _returnvalue (`|SpawnActorFromClass` "/Game/Manhattan/Characters/BP_Builder.BP_Builder_C" (`KismetMathLibrary.MakeTransform` (`self.FindAttachmentLocation` (`local.PositionId`))) "Undefined" "OverrideRootScale" null (`/Game/Manhattan/Core/Rules/BPFL_Rules.GetOccupier` (`local.Position`)) null))
      (`BlueprintMapLibrary.Map_Add` (`self.Builders`) (`local.PositionId`) _returnvalue)
      (return)
      (else
        ;[1 1 1] destroy the actor and remove it from the map
        (`self.K2_DestroyActor` (`BlueprintMapLibrary.Map_Find` (`self.Builders`) (`local.PositionId`)))
        (`BlueprintMapLibrary.Map_Remove` (`self.Builders`) (`local.PositionId`))
        (return)))))

(fn `ShowCharacters`
  (bind _sboardpositionid (`/Game/Manhattan/Core/Util/BPML_Util.ForEachPosition`)
    (:`LoopBody`
      (`|ExecutionSequence`
        (:`then_0`
          (bind _position (`/Game/Manhattan/Core/Rules/BPFL_Rules.GetPositionFromId` (`self.DisplayState`) _sboardpositionid))
          (`self.ShowBlocks` _position))
        (:`then_1`
          (`self.ShowBuilders` _position))))
    (:`Completed`
      (return))))

(fn `UserConstructionScript`
  (locals (position :type "/Game/Manhattan/Core/Data/SBoardPositionId Structure"))
  (bind (_returnvalue_location _returnvalue_rotation _returnvalue_scale) (`KismetMathLibrary.BreakTransform` (`SceneComponent.GetRelativeTransform` (`self.TopLeft`))))
  (set `self.AttachmentMap` (`|MakeMap`))
  (bind _sboardpositionid (`/Game/Manhattan/Core/Util/BPML_Util.ForEachPosition`)
    (:`LoopBody`
      (bind _output_get (set `local.position` _sboardpositionid))
      (bind _returnvalue (`AddComponent|NODE_AddArrowComponent-0` :`RelativeTransform` (`KismetMathLibrary.MakeTransform` (+ (`KismetMathLibrary.MakeVector` (* (`.Col_12_EDB32F0040193954677561AD2BC46ECB` (break `/Game/Manhattan/Core/Data/SBoardPositionId` _output_get)) 100.0) (* (break `/Game/Manhattan/Core/Data/SBoardPositionId` _output_get) 100.0)) _returnvalue_location) _returnvalue_rotation _returnvalue_scale)))
      (`BlueprintMapLibrary.Map_Add` (`self.AttachmentMap`) (`local.position`) _returnvalue))
    (:`Completed`
      (set `self.BaseAttachmentMap` (`self.AttachmentMap`)))))