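; Clickable selection indicator for a player's Builder, shown as a spinning, bobbing quad pyramid.
; A timeline drives the sine-based bob while Tick spins the mesh, both running faster when Active through hover or selection.
; Clicking an unselected indicator notifies the current controller with itself and marks it selected.
; OnSelected and OnDeselected also set the state, and the material follows the owning player and selection.
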(event `self.ReceiveBeginPlay`
  (bind (_direction _0_360) (`Timeline|Timeline`)
    (:`Update`
      (`SceneComponent.K2_SetRelativeLocation` (`self.Shape_QuadPyramid`) (`KismetMathLibrary.MakeVector` 0.0 0.0 (* (`KismetMathLibrary.DegSin` _0_360) 10.0)) false false))))

(event `self.ReceiveTick`
  (params (DeltaSeconds :type "Float (single-precision)"))
  (`SceneComponent.K2_AddRelativeRotation` (`self.Shape_QuadPyramid`) (`KismetMathLibrary.MakeRotator` 0.0 0.0 (* DeltaSeconds (select `bool` (`self.Active`) :`false` 50.0 :`true` 100.0 :!type "Float (single-precision)"))) false false))

(event `self.ReceiveActorOnClicked`
  (params (ButtonPressed :type "Key Structure"))
  (if (not (`self.Selected`))
    (`/Game/Manhattan/Core/Util/BPFL_Util.FireEventOnCurrentController` "NewEnumerator2" (struct) self)
    (set `self.Selected` true)
    (`self.UpdateColor` :!label _label)
    (`self.UpdateHover`)))

(event `OnDeselected`
  (set `self.Selected` false)
  (set `self.Active` false)
  (goto _label))

(event `OnSelected`
  (set `self.Selected` true)
  (set `self.Active` true)
  (goto _label))

(event `self.ReceiveActorBeginCursorOver`
  (set `self.Active` true)
  (`self.UpdateHover` :!label _label_2))

(event `self.ReceiveActorEndCursorOver`
  (set `self.Active` (`self.Selected`))
  (goto _label_2))

(fn `UpdateColor`
  (bind _builder_player (break `/Game/Manhattan/Core/Data/SBuilder` (`self.Builder`)))
  (switch `/Game/Manhattan/Core/Data/EPlayerId` _builder_player
    (:`NewEnumerator0`
      (`PrimitiveComponent.SetMaterial` (`self.Shape_QuadPyramid`) 0 (select `bool` (`self.Selected`) :`false` "/Game/Manhattan/Interaction/SelectionIndicator/MI_SelectionIndicator_Player1.MI_SelectionIndicator_Player1" :`true` "/Game/Manhattan/Interaction/SelectionIndicator/MI_SelectionIndicator_Player1Selected.MI_SelectionIndicator_Player1Selected" :!type "MaterialInterface Object Reference")))
    (:`NewEnumerator1`
      (`PrimitiveComponent.SetMaterial` (`self.Shape_QuadPyramid`) 0 (select `bool` (`self.Selected`) :`false` "/Game/Manhattan/Interaction/SelectionIndicator/MI_SelectionIndicator_Player2.MI_SelectionIndicator_Player2" :`true` "/Game/Manhattan/Interaction/SelectionIndicator/MI_SelectionIndicator_Player2Selected.MI_SelectionIndicator_Player2Selected" :!type "MaterialInterface Object Reference")))))

(fn `UpdateHover`
  (`TimelineComponent.SetPlayRate` (`self.Timeline`) (select `bool` (`self.Active`) :`false` 1.0 :`true` 2.0 :!type "Float (single-precision)"))
  (return))

(fn `UserConstructionScript`
  (set `self.Active` (`self.Selected`))
  (`self.UpdateColor`))