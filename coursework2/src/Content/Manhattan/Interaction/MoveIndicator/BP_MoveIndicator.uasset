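; BP_MoveIndicator is a clickable board marker for one possible Move in Manhattan, either a setup placement, a move or a build.
; The construction script picks the plane's glow material from the move type, using a per-player material for moves.
; Hovering shows the move's preview actor through the character pool, hidden again on hover end or destruction.
; Clicking fires an event carrying the Move on the current controller; click and hover-show are ignored while the camera turns.
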(event `self.ReceiveActorOnClicked`
  (params (ButtonPressed :type "Key Structure"))
  (if (not (`/Game/Manhattan/Interaction/Board/BP_Board.bCameraTurning` (`/Game/Manhattan/Core/Util/BPFL_Util.GetBoard`)))
    (`/Game/Manhattan/Core/Util/BPFL_Util.FireEventOnCurrentController` "NewEnumerator1" (`self.Move`))))

(event `self.ReceiveActorBeginCursorOver`
  (if (not (`/Game/Manhattan/Interaction/Board/BP_Board.bCameraTurning` (`/Game/Manhattan/Core/Util/BPFL_Util.GetBoard`)))
    (`/Game/Manhattan/Interaction/CharacterPool/BP_CharacterPool.ShowActorForMove` (`/Game/Manhattan/Core/Util/BPFL_Util.GetCharacterPool`) (`self.Move`))))

(event `self.ReceiveDestroyed`
  (`/Game/Manhattan/Interaction/CharacterPool/BP_CharacterPool.HideActorForMove` (`/Game/Manhattan/Core/Util/BPFL_Util.GetCharacterPool`) (`self.Move`) :!label _label))

(event `self.ReceiveActorEndCursorOver`
  (goto _label))

(fn `UserConstructionScript`
  (bind (_move_type _move_from _move_to _move_with) (break `/Game/Manhattan/Core/Data/SMove` (`self.Move`)))
  (`PrimitiveComponent.SetMaterial` (`self.Plane`) 0 (select `/Game/Manhattan/Core/Data/EMoveType` _move_type :`NewEnumerator0` "/Game/Manhattan/Interaction/MoveIndicator/MI_Glow_Setup.MI_Glow_Setup" :`NewEnumerator1` (select `/Game/Manhattan/Core/Data/EPlayerId` (`.Player_7_C4F68868479E4B5066DA7C85D82F0A0D` (break `/Game/Manhattan/Core/Data/SBuilder` _move_with)) :`NewEnumerator0` "/Game/Manhattan/Interaction/MoveIndicator/MI_Glow_Move_Player1.MI_Glow_Move_Player1" :`NewEnumerator1` "/Game/Manhattan/Interaction/MoveIndicator/MI_Glow_Move_Player2.MI_Glow_Move_Player2" :!type "MaterialInterface Object Reference") :`NewEnumerator2` "/Game/Manhattan/Interaction/MoveIndicator/MI_Glow_Build.MI_Glow_Build")))