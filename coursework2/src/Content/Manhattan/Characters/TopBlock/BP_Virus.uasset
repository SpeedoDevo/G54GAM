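; BP_Virus is a decorative virus actor that bobs up and down at a random spot inside its bounding box.
; On BeginPlay it moves its Scene component to a random point in the box and picks a random amplitude.
; A timeline with random play rate and start point drives a sine offset on the Virus component's Z, so instances move out of sync.
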(event `self.ReceiveBeginPlay`
  (bind _boundingbox (`self.BoundingBox`))
  (`|ExecutionSequence`
    (:`then_0`
      ;[1 1 1] find a random location
      (`SceneComponent.K2_SetRelativeLocation` (`self.Scene`) (`KismetMathLibrary.RandomPointInBoundingBox` (`SceneComponent.RelativeLocation` _boundingbox) (`BoxComponent.BoxExtent` _boundingbox)) false false))
    (:`then_1`
      (set `self.Amplitude` (`KismetMathLibrary.RandomFloatInRange` 5.0 10.0)))
    (:`then_2`
      ;[1 1 1] set a random pace for the motion
      (`TimelineComponent.SetPlayRate` (`self.Timeline`) (`KismetMathLibrary.RandomFloatInRange` 0.1 1.0)))
    (:`then_3`
      (bind (_direction _0_360) (`Timeline|Timeline` :`NewTime` (`KismetMathLibrary.RandomFloat`) :!via `SetNewTime` :!label _label)
        (:`Update`
          ;[1 1 1] do the motion
          (`SceneComponent.K2_SetRelativeLocation` (`self.Virus`) (`KismetMathLibrary.MakeVector` 0.0 0.0 (* (`KismetMathLibrary.DegSin` _0_360) (`self.Amplitude`))) false false))))
    (:`then_4`
      (goto _label))))

(fn `UserConstructionScript`)