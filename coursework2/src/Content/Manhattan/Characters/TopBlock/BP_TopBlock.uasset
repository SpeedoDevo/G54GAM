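; BP_TopBlock is a character asset that hosts three BP_Virus child actors, each confined to its own box.
; The construction script calls SetVirusBox for each virus, casting the child actor to BP_Virus and assigning its matching bounding box.
; Each virus then picks random locations within that box, according to the author's comment.
; An older inline version of that assignment remains unconnected.
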(fn `SetVirusBox`
  (params (VirusChildActorComponent :type "ChildActorComponent Object Reference") (BoundingBox :type "BoxComponent Object Reference"))
  (bind _asbp_virus (cast `/Game/Manhattan/Characters/TopBlock/BP_Virus` (`ChildActorComponent.ChildActor` VirusChildActorComponent)))
  (set `/Game/Manhattan/Characters/TopBlock/BP_Virus.BoundingBox` BoundingBox _asbp_virus)
  (return))

(fn `UserConstructionScript`
  ;[1 1 1] assign each virus their own bounding box (they will randomly find a location within the box)
  (`self.SetVirusBox` (`self.Virus0`) (`self.Box0`))
  (`self.SetVirusBox` (`self.Virus1`) (`self.Box1`))
  (`self.SetVirusBox` (`self.Virus2`) (`self.Box2`)))