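; BP_SmartBlock is a building block actor that picks its block type from its Height.
; The construction script calls UpdateHeight, which swaps the ChildActor component's class between BP_TopBlock for heights above 3 and BP_Block otherwise.
; A regular block receives the height and exposes its Attachment, while a top block clears Attachment and HasAttachment.
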(fn `UpdateHeight`
  (params (Height :type Integer :default 0))
  (bind _childactor (`self.ChildActor`))
  ;[1 1 1] is top block
  (bind _output_get (set `self.Height` Height))
  (if (> _output_get 3)
    ;[1 1 1] top block has no attachment
    (`ChildActorComponent.SetChildActorClass` (`self.ChildActor`) "/Game/Manhattan/Characters/TopBlock/BP_TopBlock.BP_TopBlock_C")
    (set `self.bHasAttachment` false)
    (set `self.Attachment` null)
    (else
      ;[1 1 1] regular block has attachment
      (`ChildActorComponent.SetChildActorClass` _childactor "/Game/Manhattan/Characters/BP_Block.BP_Block_C")
      (bind _asbp_block (cast `/Game/Manhattan/Characters/BP_Block` (`ChildActorComponent.ChildActor` _childactor)))
      (`/Game/Manhattan/Characters/BP_Block.UpdateHeight` _asbp_block (`self.Height`))
      (set `self.bHasAttachment` true)
      (set `self.Attachment` (`/Game/Manhattan/Characters/BP_Block.Attachment` _asbp_block)))))

(fn `UserConstructionScript`
  (`self.UpdateHeight` (`self.Height`)))