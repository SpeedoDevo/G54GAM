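; BP_Block is a block actor in the Manhattan game whose appearance reflects its Height level.
; UpdateHeight stores the level, picks a material and a progressively smaller uniform scale for higher levels, and falls back to a full-size wall look otherwise.
; It then applies the material to the Cube and the scale to the root component.
; The construction script runs the same function, so the look follows Height at construction.
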(fn `UpdateHeight`
  (params (Height :type Integer))
  (locals (Material :type "Material Object Reference") (Scale :type "Vector Structure"))
  (bind _returnvalue (`KismetMathLibrary.MakeVector` 1.0 1.0 1.0))
  (set `self.Height` Height)
  (`|ExecutionSequence`
    (:`then_0`
      ;[1 1 1] set the scale and material varaibales based on height
      (switch `int` (`self.Height`)
        (:`Default`
          (set `local.Material` "/Game/StarterContent/Materials/M_Basic_Wall.M_Basic_Wall")
          (set `local.Scale` _returnvalue))
        (:`1`
          (set `local.Material` "/Game/StarterContent/Materials/M_Metal_Rust.M_Metal_Rust")
          (set `local.Scale` (* _returnvalue 0.9)))
        (:`2`
          (set `local.Material` "/Game/StarterContent/Materials/M_Metal_Steel.M_Metal_Steel")
          (set `local.Scale` (* _returnvalue 0.8)))
        (:`3`
          (set `local.Material` "/Game/StarterContent/Materials/M_Metal_Gold.M_Metal_Gold")
          (set `local.Scale` (* _returnvalue 0.7)))))
    (:`then_1`
      ;[1 1 1] propagate the variables to the proper targets
      (`PrimitiveComponent.SetMaterial` (`self.Cube`) 0 (`local.Material`))
      (`SceneComponent.SetRelativeScale3D` (`self.DefaultSceneRoot`) (`local.Scale`)))))

(fn `UserConstructionScript`
  (`self.UpdateHeight` (`self.Height`)))